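; BP_AreaClear is a level progression actor that opens new areas as enemy waves are cleared.
; On BeginPlay it binds to OnAllWavesCompleted on each referenced wave manager.
; HandleWaveCompleted finds the sender's array index and, through a hardcoded switch, destroys the matching blocking wall for the second area, third area or extraction site.
; It then updates the player controller's objective text to point onward.
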(event Custom|OnAllWavesCompleted_Event
  (params (ObjSender :type BP%20Wave%20Manager%20Object%20Reference))
  (CallFunction|HandleWaveCompleted ObjSender))

(event EventBeginPlay
  (for _array_element (Variables|Default|GetWaveManagers)
    (EventDispatchers|AssignOnAllWavesCompleted _array_element (delegate Custom|OnAllWavesCompleted_Event))))

(event Collision|EventActorBeginOverlap
  (params (OtherActor :type Actor%20Object%20Reference)))

(event EventTick
  (params (DeltaSeconds :type Float%20%28single-precision%29)))

(fn ConstructionScript)

(fn HandleWaveCompleted
  (params (objSender :type BP%20Wave%20Manager%20Object%20Reference))
  ;[0.15 0.15 0.15 0.5] Going to perform some bad practices for the sake of getting this done...
  (LocalVariables|SetindexOfWaveManager 0)
  (for (_array_element _array_index) (Variables|Default|GetWaveManagers)
    (if (== _array_element objSender)
      (LocalVariables|SetindexOfWaveManager _array_index)))
  (switch int (LocalVariables|GetindexOfWaveManager)
    (:0
      ;[0.15 0.15 0.15 0.5] Handle Starting wave completed
      (Actor|DestroyActor (Variables|Default|GetWallBlockingSecondArea))
      (bind _returnvalue (Actor|GetActorOfClass "/Game/FirstPerson/Blueprints/BP_FirstPersonPlayerController.BP_FirstPersonPlayerController_C"))
      (Default|SetCanvasObjectiveText _returnvalue (Variables|Default|GetMoveToAreaObjectiveText)))
    (:1
      ;[0.15 0.15 0.15 0.5] Handle Second Wave Complete
      (Actor|DestroyActor (Variables|Default|GetWallBlockingThirdArea))
      (bind _returnvalue_2 (Actor|GetActorOfClass "/Game/FirstPerson/Blueprints/BP_FirstPersonPlayerController.BP_FirstPersonPlayerController_C"))
      (Default|SetCanvasObjectiveText _returnvalue_2 (Variables|Default|GetMoveToAreaObjectiveText)))
    (:2
      (Actor|DestroyActor (Variables|Default|GetWallBlockingExtractionSite))
      (bind _returnvalue_3 (Actor|GetActorOfClass "/Game/FirstPerson/Blueprints/BP_FirstPersonPlayerController.BP_FirstPersonPlayerController_C"))
      (Default|SetCanvasObjectiveText _returnvalue_3 (Variables|Default|GetHeadToExtractionText)))))