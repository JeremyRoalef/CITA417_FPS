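; Wave manager that spawns timed waves of AI enemies at BP_SpawnPoint actors, starting on BeginPlay or when a wave area is entered.
; SpawnEnemy recursively walks each wave's enemy list, delaying before each spawn at the first available point and retrying every second when none is free.
; A wave completes once its last enemy spawns, not when enemies die.
; After a delay it starts the next wave or signals all waves completed.
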(event Custom|SpawnWave
  (params (WaveIndex :type Integer))
  (if (Utilities|Array|IsValidIndex (Variables|Components|GetWaves) WaveIndex)
    (Development|PrintString "Looping over enemies to spawn")
    (CallFunction|SpawnEnemy 0 WaveIndex)
    (else
      (Development|PrintString "Wave index is invalid"))))

(event Custom|OnWaveComplete
  (Utilities|FlowControl|Delay (Variables|Default|GetDelayBetweenWaves))
  (bind _nextwaveexists (CallFunction|CanGetNextWave))
  (if _nextwaveexists
    (bind _result (Math|Integer|IncrementInt (Variables|Default|GetcurrentWaveIndex))
      (:%20%20
        (bind _output_get (Variables|Default|SetcurrentWaveIndex _result))
        (CallFunction|SpawnWave _output_get)))
    (else
      (CallFunction|OnAllWavesComplete))))

(event Custom|OnAllWavesComplete
  (Development|PrintString "All waves in level complete")
  (Default|CallOnAllWavesCompleted self))

(event Custom|SpawnEnemy
  (params (index :type Integer) (waveIndex :type Integer))
  (bind _returnvalue (+ index 1))
  (bind _waves (Variables|Components|GetWaves))
  (bind _output (Utilities|Array|Get(acopy) _waves waveIndex))
  (bind _enemiestospawn (Variables|/Game/Spawning/Waves/BP_WaveData.BP_WaveData_C|GetEnemiesToSpawn _output))
  (bind _spawndelay (Variables|/Game/Spawning/Waves/BP_WaveData.BP_WaveData_C|GetSpawnDelay _output))
  ;[0.15 0.15 0.15 0.5] This looks terrible
  (if (Utilities|Array|IsValidIndex _enemiestospawn index)
    (bind (_receivedspawnpoint _spawnpoint) (CallFunction|TryGetAvailableSpawnPoint))
    (if _receivedspawnpoint
      (Development|PrintString (Utilities|String|ToString(Float) _spawndelay))
      (Utilities|FlowControl|Delay _spawndelay)
      (AI|SpawnAIFromClass (Utilities|Array|Get(acopy) _enemiestospawn index) 0 (+ _spawnpoint (Math|Vector|MakeVector 0.0 0.0 (Variables|Default|GetSpawnHeightOffset))) "0, 0, 0" false 0)
      (if (Utilities|Array|IsValidIndex _enemiestospawn _returnvalue)
        (CallFunction|SpawnEnemy _returnvalue waveIndex)
        (else
          (CallFunction|OnWaveComplete)))
      (else
        (Utilities|FlowControl|Delay 1.0)
        (CallFunction|SpawnEnemy index waveIndex)))
    (else
      (Development|PrintString "No enemy to spawn")
      (CallFunction|OnWaveComplete))))

(event Custom|OnWaveAreaEntered
  (if (not (Variables|Default|GetisStarted))
    (Variables|Default|SetisStarted true)
    (CallFunction|SpawnWave (stale EventBeginPlay _output_get))))

(event EventBeginPlay
  (CallFunction|SetSpawnPointsinScene)
  (bind _output_get (Variables|Default|SetcurrentWaveIndex 0))
  (Development|PrintString "Got all spawn points")
  (if (Variables|Default|GettriggerOnStart)
    (Variables|Default|SetisStarted true)
    (CallFunction|SpawnWave _output_get)))

(fn ConstructionScript)

(fn SetSpawnPointsinScene
  (bind _outactors (Actor|GetAllActorsOfClass "/Game/Spawning/BP_SpawnPoint.BP_SpawnPoint_C"))
  (Variables|Default|SetSpawnPoints _outactors))

(fn TryGetAvailableSpawnPoint
  (for _array_element (Variables|Default|GetSpawnPoints)
    (if (Variables|/Game/Spawning/BP_SpawnPoint.BP_SpawnPoint_C|GetisAvailable _array_element)
      (return true (Transformation|GetActorLocation _array_element))))
  (return false "0, 0, 0"))

(fn CanGetNextWave
  (return (Utilities|Array|IsValidIndex (Variables|Components|GetWaves) (+ (Variables|Default|GetcurrentWaveIndex) 1))))